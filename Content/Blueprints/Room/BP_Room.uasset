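; Room actor that builds a randomized grid arena and places one player and one AI at game start.
; Obstacles come from the pool manager by per-cell chance and mark a 2D busy-cell map, which is rebuilt on each start.
; Spawning picks a random free cell by recursive retry.
; Game-mode tick, during one game state, clamps registered characters inside the room borders.
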(event Custom|ED_StartGame
  (if (Utilities|Enum|Equal(Enum) (CallFunction|BPFLGetGameState) "NewEnumerator2")
    (CallFunction|FRegenerateObstacles)
    (CallFunction|FSpawnCharacter true)
    (CallFunction|FSpawnCharacter false)))

(event Custom|ED_Tick
  (params (GameState :type E_GameState%20Enum :default "NewEnumerator0"))
  (if (Utilities|Enum|Equal(Enum) GameState "NewEnumerator2")
    (Characters|FControlBorders)))

(event EventBeginPlay
  (Main|FInit (delegate Custom|ED_Tick) (delegate Custom|ED_StartGame)))

(event EventEndPlay
  (params (EndPlayReason :type EEndPlayReason%20Enum :default "Destroyed"))
  (Main|FDeinit (delegate Custom|ED_Tick)))

(fn ConstructionScript)

(fn FInit
  (params (ED_TIck :type Delegate%20%28by%20ref%29) (ED_StartGame :type Delegate%20%28by%20ref%29))
  (Obstacles|FGenerateObstacles)
  (Default|FSubscribeTick (CallFunction|BPFLGetGameMode) ED_TIck)
  (Default|FSubscribeStartGame (CallFunction|BPFLGetHUD) ED_StartGame))

(fn FGenerateObstacles
  (bind _cells (Variables|Obstacles|GetCells))
  (bind _step (Variables|Obstacles|GetStep))
  (bind _busycells (Variables|Obstacles|GetBusyCells))
  (bind _busycells_2 (Variables|Obstacles|GetBusyCells))
  (bind _spawnpoint (Variables|Default|GetSpawnPoint))
  (bind _returnvalue (Math|Float|Truncate (.x _cells)))
  (bind _returnvalue_2 (Math|Float|Truncate (.y _cells)))
  (bind _returnvalue_3 (Transformation|GetWorldLocation _spawnpoint))
  (Utilities|Array|Resize _busycells_2 (+ _returnvalue 1))
  (for (_ _array_index) _busycells_2
    (Utilities|Array|Resize (Utilities|Struct|BreakSTR_BusyCells (Utilities|Array|Get(acopy) _busycells_2 _array_index)) (+ _returnvalue_2 1))
    (Utilities|Array|SetArrayElem _busycells_2 _array_index (Utilities|Struct|MakeSTR_BusyCells (Utilities|Struct|BreakSTR_BusyCells (Utilities|Array|Get(acopy) _busycells_2 _array_index)))))
  (for _index (range 0 _returnvalue)
    (for _index_2 (range 0 _returnvalue_2)
      (if (<= (Math|Random|RandomFloatinRange 0.0 1.0) (Variables|Obstacles|GetGenerationChance))
        (bind _return (Default|FGetPoolObject (CallFunction|BPFLGetPoolManager) (Variables|Obstacles|GetObstacle) (Math|Vector|MakeVector (+ (.x _returnvalue_3) (* _index _step)) (+ (* _index_2 _step) (.y _returnvalue_3)) 0.0) "0, 0, 0"))
        (bind _asbp_obstacle (Utilities|Casting|CastToBP_Obstacle _return))
        (Utilities|Array|Add (Variables|Obstacles|GetObstacles) _asbp_obstacle)
        (Utilities|Array|SetArrayElem (.isbusycells (Utilities|Array|Get(acopy) _busycells _index)) _index_2 true)
        (Utilities|Array|SetArrayElem _busycells _index (Utilities|Struct|MakeSTR_BusyCells (.isbusycells (Utilities|Array|Get(acopy) _busycells _index))))))))

(fn FAddCharacter
  (params (Character :type BP%20Character%20Object%20Reference%20%28by%20ref%29))
  (Utilities|Array|AddUnique (Variables|Characters|GetCharacters) Character))

(fn FRemoveCharacter
  (params (Character :type BP%20Character%20Object%20Reference%20%28by%20ref%29))
  (Utilities|Array|RemoveItem (Variables|Characters|GetCharacters) Character))

(fn FRemoveAllCharacter
  (Utilities|Array|Clear (Variables|Characters|GetCharacters)))

(fn FDeinit
  (params (ED_Tick :type Delegate%20%28by%20ref%29))
  (Characters|FRemoveAllCharacter)
  (Default|FUnsubscribeTick (CallFunction|BPFLGetGameMode) ED_Tick))

(fn FControlBorders
  (bind _borders (Variables|Characters|GetBorders))
  (for _array_element (Variables|Characters|GetCharacters)
    (if (or (or (<= (Math|Float|Clamp(Float) (.x (Transformation|GetActorLocation _array_element)) (.x _borders) (.z _borders)) (.x _borders)) (>= (Math|Float|Clamp(Float) (.x (Transformation|GetActorLocation _array_element)) (.x _borders) (.z _borders)) (.z _borders))) (or (<= (Math|Float|Clamp(Float) (.y (Transformation|GetActorLocation _array_element)) (.y _borders) (.w _borders)) (.y _borders)) (>= (Math|Float|Clamp(Float) (.y (Transformation|GetActorLocation _array_element)) (.y _borders) (.w _borders)) (.w _borders))))
      (Transformation|SetActorLocation _array_element (Math|Vector|MakeVector (Math|Float|Clamp(Float) (.x (Transformation|GetActorLocation _array_element)) (.x _borders) (.z _borders)) (Math|Float|Clamp(Float) (.y (Transformation|GetActorLocation _array_element)) (.y _borders) (.w _borders)) (.z (Transformation|GetActorLocation _array_element))) true false))))

(fn FSpawnCharacter
  (params (isPlayer :type Boolean))
  (bind _returnvalue (Math|Transform|MakeTransform "0, 0,10.000000" "0, 0, 0" "1.750000,1.750000,1.750000"))
  (bind _step (Variables|Obstacles|GetStep))
  (bind _spawnpoint (Variables|Default|GetSpawnPoint))
  (bind _returnvalue_2 (Transformation|GetWorldLocation _spawnpoint))
  (if isPlayer
    (bind _returnvalue_3 (Game|SpawnActorfromClass (Variables|Characters|GetPlayer) _returnvalue "AlwaysSpawn" 0 0))
    (LocalVariables|SetSpawnedActor _returnvalue_3)
    (else
      (bind _returnvalue_4 (Game|SpawnActorfromClass (Variables|Characters|GetAI) _returnvalue "AlwaysSpawn" 0 0))
      (LocalVariables|SetSpawnedActor _returnvalue_4)))
  (bind (_x _y) (CallFunction|FSearchFreeCellSpawn))
  (Transformation|SetActorLocation (LocalVariables|GetSpawnedActor) (Math|Vector|MakeVector (+ (.x _returnvalue_2) (* _x _step)) (+ (* _y _step) (.y _returnvalue_2)) 0.0) false true)
  (return (LocalVariables|GetSpawnedActor)))

(fn FSearchFreeCellSpawn
  (for (_array_element _array_index) (Variables|Obstacles|GetBusyCells)
    (if (>= (Math|Random|RandomFloatinRange 0.0 1.0) 0.9)
      (for (_array_element_2 _array_index_2) (Utilities|Struct|BreakSTR_BusyCells _array_element)
        (if (not _array_element_2)
          (if (>= (Math|Random|RandomFloatinRange 0.0 1.0) 0.9)
            (return _array_index _array_index_2))))))
  (bind (_x _y) (CallFunction|FSearchFreeCellSpawn))
  (return _x _y))

(fn FGetIndexObstacle
  (params (Obstacle :type BP%20Obstacle%20Object%20Reference))
  (return (Utilities|Array|FindItem (Variables|Obstacles|GetObstacles) Obstacle)))

(fn FRegenerateObstacles
  (bind _busycells (Variables|Obstacles|GetBusyCells))
  (for _array_element (Variables|Obstacles|GetObstacles)
    (Default|FSetActive _array_element false))
  (for (_ _array_index) _busycells
    (for (_ _array_index_2) (.isbusycells (Utilities|Array|Get(acopy) _busycells _array_index))
      (Utilities|Array|SetArrayElem (.isbusycells (Utilities|Array|Get(acopy) _busycells _array_index)) _array_index_2 false))
    (Utilities|Array|SetArrayElem (Variables|Obstacles|GetBusyCells) _array_index (Utilities|Struct|MakeSTR_BusyCells (.isbusycells (Utilities|Array|Get(acopy) _busycells _array_index)))))
  (Obstacles|FGenerateObstacles))