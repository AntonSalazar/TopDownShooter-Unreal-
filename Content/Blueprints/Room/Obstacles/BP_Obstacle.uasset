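; BP_Obstacle is a room obstacle that oscillates vertically and deactivates whizbang projectiles that overlap its box.
; It moves on a game-mode tick subscription during two game states, bouncing a clamped timer between height offsets at a speed randomized on BeginPlay.
; An activation event toggles collision on the box and mesh.
; Character overlaps are detected but trigger no action.
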(event OnComponentBeginOverlap(Box)
  (params (OverlappedComponent :type Primitive%20Component%20Object%20Reference) (OtherActor :type Actor%20Object%20Reference) (OtherComp :type Primitive%20Component%20Object%20Reference) (OtherBodyIndex :type Integer) (bFromSweep :type Boolean) (SweepResult :type Hit%20Result%20Structure%20%28by%20ref%29))
  (if (Utilities|ClassIsChildOf (Utilities|GetClass OtherActor) "/Game/Blueprints/Character/Base/BP_Character.BP_Character_C")
    (Utilities|Casting|CastToBP_Character OtherActor)
    (else
      (bind _asbp_whizbang_model (Utilities|Casting|CastToBP_WhizbangModel OtherActor))
      (Default|FSetActive _asbp_whizbang_model false))))

(event Custom|ED_Activate
  (params (isActive :type Boolean))
  (bind _box (Variables|Default|GetBox))
  (if isActive
    (if (Utilities|Enum|NotEqual(Enum) (Collision|GetCollisionEnabled _box) "QueryAndPhysics")
      (Collision|SetCollisionEnabled (Variables|Default|GetBox) "QueryAndPhysics")
      (Collision|SetCollisionEnabled (Variables|Default|GetMesh) "QueryAndPhysics"))
    (elif (Utilities|Enum|NotEqual(Enum) (Collision|GetCollisionEnabled _box) "NoCollision")
      (Collision|SetCollisionEnabled (Variables|Default|GetBox) "NoCollision")
      (Collision|SetCollisionEnabled (Variables|Default|GetMesh) "NoCollision"))))

(event Custom|ED_Tick
  (params (GameState :type E_GameState%20Enum :default "NewEnumerator0"))
  (if (or (Utilities|Enum|Equal(Enum) GameState "NewEnumerator0") (Utilities|Enum|Equal(Enum) GameState "NewEnumerator2"))
    (CallFunction|FMovement)))

(event EventBeginPlay
  (|CallParentFunction)
  (Default|FSubscribeTick (CallFunction|BPFLGetGameMode) (delegate Custom|ED_Tick))
  (CallFunction|FSubscribeActive (delegate Custom|ED_Activate))
  (CallFunction|FInit))

(event EventEndPlay
  (params (EndPlayReason :type EEndPlayReason%20Enum :default "Destroyed"))
  (|CallParentFunction EndPlayReason)
  (Default|FUnsubscribeTick (CallFunction|BPFLGetGameMode) (delegate Custom|ED_Tick))
  (CallFunction|FSubscribeActive (delegate Custom|ED_Activate)))

(fn ConstructionScript)

(fn FMovement
  (bind _returnvalue (Transformation|GetActorLocation))
  (bind _heightoffset (Variables|ObstacleSettings|GetHeightOffset))
  (CallFunction|FTiming)
  (Transformation|SetActorRelativeLocation (Math|Vector|MakeVector (.x _returnvalue) (.y _returnvalue) (Math|Float|MapRangeClamped (Variables|ObstacleSettings|GetTimer) 0.0 1.0 (.x _heightoffset) (.y _heightoffset))) true))

(fn FInit
  (Variables|ObstacleSettings|SetTimeOffset (Math|Vector|MakeVector (.x (Variables|ObstacleSettings|GetTimeOffset)) (Math|Random|RandomFloatinRange (.x (Variables|ObstacleSettings|GetTimeOffset)) (.z (Variables|ObstacleSettings|GetTimeOffset))) (.z (Variables|ObstacleSettings|GetTimeOffset)))))

(fn FTiming
  (bind _output_get (Variables|ObstacleSettings|SetTimer (Math|Float|Clamp(Float) (+ (* (Utilities|Time|GetWorldDeltaSeconds) (.y (Variables|ObstacleSettings|GetTimeOffset)) (Variables|ObstacleSettings|GetSign)) (Variables|ObstacleSettings|GetTimer)))))
  (if (or (== _output_get 0.0) (== _output_get 1.0))
    (Variables|ObstacleSettings|SetSign (* (Variables|ObstacleSettings|GetSign) -1.0))))