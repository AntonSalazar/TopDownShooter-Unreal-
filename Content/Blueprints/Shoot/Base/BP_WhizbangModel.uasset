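; Base shell projectile that kills opposing characters, scores for its owner and ricochets off other objects.
; Init sets the owner side and picks speed from game difficulty.
; A life-cycle dispatcher drives swept forward movement or deactivates the shell, depending on game state.
; Each step deactivates it outside the XY life zone, otherwise line-traces ahead for WorldDynamic hits, mirroring direction with a random sound on non-character impacts.
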(event Custom|ED_LifeTime
  (params (GameState :type E_GameState%20Enum :default "NewEnumerator0"))
  (if (Utilities|Enum|Equal(Enum) GameState "NewEnumerator2")
    (CallFunction|FMovement)
    (elif (Utilities|Enum|Equal(Enum) GameState "NewEnumerator0")
      (CallFunction|FSetActive false))))

(event EventBeginPlay
  (|CallParentFunction)
  (CallFunction|FSubscribeLifeCicle (delegate Custom|ED_LifeTime)))

(event EventEndPlay
  (params (EndPlayReason :type EEndPlayReason%20Enum :default "Destroyed"))
  (|CallParentFunction EndPlayReason)
  (CallFunction|FUnsubscribeLifeCicle (delegate Custom|ED_LifeTime)))

(event EventDestroyed
  (|CallParentFunction)
  (CallFunction|FUnsubscribeLifeCicle (delegate Custom|ED_LifeTime)))

(fn ConstructionScript
  (|CallParentFunction))

(fn FMovement
  (bind _returnvalue (Utilities|Time|GetWorldDeltaSeconds))
  (bind _returnvalue_2 (Transformation|GetActorLocation))
  (bind _returnvalue_3 (Transformation|GetActorLocation))
  (bind _returnvalue_4 (Transformation|GetActorForwardVector))
  (bind _movespeed (Variables|Default|GetMoveSpeed))
  (bind _lifezone (Variables|Default|GetLifeZone))
  (bind _hitsounds (Variables|Default|GetHitSounds))
  (bind _returnvalue_5 (Math|Float|Clamp(Float) (.y _returnvalue_3) (.y _lifezone) (.w _lifezone)))
  (bind _returnvalue_6 (Math|Float|Clamp(Float) (.x _returnvalue_3) (.x _lifezone) (.z _lifezone)))
  (bind _returnvalue_7 (* _movespeed _returnvalue))
  (bind _returnvalue_8 (* _returnvalue_4 _returnvalue_7))
  (Transformation|AddActorWorldOffset _returnvalue_8 true)
  (if (or (or (<= _returnvalue_6 (.x _lifezone)) (>= _returnvalue_6 (.z _lifezone))) (or (<= _returnvalue_5 (.y _lifezone)) (>= _returnvalue_5 (.w _lifezone))))
    (CallFunction|FSetActive false)
    (else
      (bind (_outhit _returnvalue_9) (Collision|LineTraceForObjects _returnvalue_2 (+ _returnvalue_2 _returnvalue_8) (Utilities|Array|MakeArray "ObjectTypeQuery2") false 0 "None"))
      (if _returnvalue_9
        (bind _asbp_character (Utilities|Casting|CastToBP_Character (.HitActor (Collision|BreakHitResult _outhit)))
          (:then
            (if (Math|Boolean|NotEqual(Boolean) (Default|FIsPlayer _asbp_character) (Variables|Default|GetisPlayerOwner))
              (Default|EventDie _asbp_character)
              (CallFunction|FSetActive false)
              (CallFunction|BPFLSetScore 1 (Variables|Default|GetisPlayerOwner))))
          (:CastFailed
            (Audio|PlaySound2D (Utilities|Array|Get(acopy) _hitsounds (Math|Random|RandomInteger (- (Utilities|Array|Length _hitsounds) 1))) 1.5)
            (Transformation|SetActorRotation (Math|Rotator|FindLookatRotation (+ (.Normal (Collision|BreakHitResult _outhit)) (.ImpactPoint (Collision|BreakHitResult _outhit))) (+ (.ImpactPoint (Collision|BreakHitResult _outhit)) (Math|Vector|MirrorVectorbyNormal (* (Transformation|GetActorForwardVector) (Variables|Default|GetMoveSpeed)) (.ImpactNormal (Collision|BreakHitResult _outhit))))))))))))

(fn FInit
  (params (IgnoreActor :type Actor%20Object%20Reference) (isPlayerOwner :type Boolean))
  (Variables|Default|SetIgnoreActor IgnoreActor)
  (Variables|Default|SetisPlayerOwner isPlayerOwner)
  (switch Utilities|FlowControl|Switch|SwitchonE_GameDifficile (CallFunction|BPFLGetGameDifficult)
    (:NewEnumerator0
      (Variables|Default|SetMoveSpeed 2e+03))
    (:NewEnumerator1
      (Variables|Default|SetMoveSpeed 2.5e+03))
    (:NewEnumerator2
      (Variables|Default|SetMoveSpeed 3e+03))))