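; Shoot actor, apparently a projectile, with a sphere that can be switched on or off and colored for player or AI.
; It subscribes to an active-state event on BeginPlay and unsubscribes on EndPlay or Destroyed.
; That event toggles the sphere's collision between query-and-physics and none, changing it only when needed.
; F_SetMaterial applies the player or AI material to the sphere.
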(event Custom|ED_Activate
  (params (isActive :type Boolean))
  (bind _sphere (Variables|Default|GetSphere))
  (if isActive
    (if (Utilities|Enum|NotEqual(Enum) (Collision|GetCollisionEnabled _sphere) "QueryAndPhysics")
      (Collision|SetCollisionEnabled (Variables|Default|GetSphere) "QueryAndPhysics"))
    (elif (Utilities|Enum|NotEqual(Enum) (Collision|GetCollisionEnabled _sphere) "NoCollision")
      (Collision|SetCollisionEnabled (Variables|Default|GetSphere) "NoCollision"))))

(event EventBeginPlay
  (|CallParentFunction)
  (CallFunction|FSubscribeActive (delegate Custom|ED_Activate)))

(event EventEndPlay
  (params (EndPlayReason :type EEndPlayReason%20Enum :default "Destroyed"))
  (|CallParentFunction EndPlayReason)
  (CallFunction|FUnsubscribeActive (delegate Custom|ED_Activate)))

(event EventDestroyed
  (|CallParentFunction)
  (CallFunction|FUnsubscribeActive (delegate Custom|ED_Activate)))

(fn ConstructionScript
  (|CallParentFunction))

(fn FSetMaterial
  (params (isPlayer :type Boolean))
  (if isPlayer
    (Variables|Default|SetMaterial "/Game/GameResources/Materials/Shoot/MI_ShootPlayer.MI_ShootPlayer")
    (else
      (Variables|Default|SetMaterial "/Game/GameResources/Materials/Shoot/MI_ShootAI.MI_ShootAI")))
  (Rendering|Material|SetMaterial (Variables|Default|GetSphere) 0 (Variables|Default|GetMaterial)))