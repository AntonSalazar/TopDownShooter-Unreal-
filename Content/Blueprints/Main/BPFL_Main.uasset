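; Blueprint function library giving global shortcuts to the game's main framework objects: GM_Main, BP_GameInstance and BP_HUD.
; Wrappers forward debug flag, difficulty and game state access to the game mode, and score updates to player 0's HUD.
; Pool manager and room getters lazily find the first actor of their class, caching it on the game instance and game mode respectively.
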(fn BPFLGetGameMode
  (bind _asgm_main (Utilities|Casting|CastToGM_Main (Game|GetGameMode)))
  (return _asgm_main))

(fn BPFLIsDebug
  (return (Default|FIsDebug (CallFunction|BPFLGetGameMode))))

(fn BPFLGetGameInstance
  (bind _asbp_game_instance (Utilities|Casting|CastToBP_GameInstance (Game|GetGameInstance)))
  (return _asbp_game_instance))

(fn BPFLGetPoolManager
  (bind _bp_game_instance (CallFunction|BPFLGetGameInstance))
  (bind _poolmanager (Default|FGetPoolManager _bp_game_instance))
  (if (== _poolmanager 0)
    (bind _outactors (Actor|GetAllActorsOfClass 0 "/Game/Blueprints/Pooling/BP_PoolManager.BP_PoolManager_C"))
    (Default|FSetPoolManager _bp_game_instance (Utilities|Array|Get(acopy) _outactors))
    (return (Utilities|Array|Get(acopy) _outactors))
    (else
      (return _poolmanager))))

(fn BPFLGetRoom
  (bind _gm_main (CallFunction|BPFLGetGameMode))
  (bind _room (Default|FGetRoom _gm_main))
  (if (== _room 0)
    (bind _outactors (Actor|GetAllActorsOfClass 0 "/Game/Blueprints/Room/BP_Room.BP_Room_C"))
    (Default|FSetRoom (CallFunction|BPFLGetGameMode) (Utilities|Array|Get(acopy) _outactors))
    (return (Utilities|Array|Get(acopy) _outactors))
    (else
      (return _room))))

(fn BPFLGetHUD
  (params (PlayerIndex :type Integer))
  (bind _asbp_hud (Utilities|Casting|CastToBP_HUD (HUD|GetHUD (Game|GetPlayerController 0 PlayerIndex))))
  (return _asbp_hud))

(fn BPFLSetScore
  (params (Score :type Integer) (isPlayer :type Boolean))
  (Default|FSetScore (CallFunction|BPFLGetHUD) Score isPlayer))

(fn BPFLGetGameDifficult
  (return (Default|FGetGameDifficult (CallFunction|BPFLGetGameMode))))

(fn BPFLGetGameState
  (return (Default|FGetGameState (CallFunction|BPFLGetGameMode))))

(fn BPFLSetGameState
  (params (GameState :type E_GameState%20Enum :default "NewEnumerator0"))
  (Default|FSetGameState (CallFunction|BPFLGetGameMode) GameState))