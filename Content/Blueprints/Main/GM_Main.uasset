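; GM_Main is the main game mode, holding room, difficulty, game state and debug flag behind getter and setter functions.
; On BeginPlay it destroys CameraActors not tagged GameplayCamera and starts looping random music.
; Tick broadcasts the current state through an event dispatcher that other objects can subscribe to, cleared on EndPlay.
; The music loop's delay uses a separately randomized track's duration, so it may not match the playing track.
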(event EventBeginPlay
  (CallFunction|FInit)
  (Utilities|MPlayMusic true))

(event EventTick
  (params (DeltaSeconds :type Float%20%28single-precision%29))
  (Default|CallEDTimeTick (Variables|Default|GetState)))

(event EventEndPlay
  (params (EndPlayReason :type EEndPlayReason%20Enum :default "Destroyed"))
  (ED_Tick|FUnsubscribeAllTick))

(fn ConstructionScript)

(fn FSubscribeTick
  (params (Event :type Delegate%20%28by%20ref%29))
  (EventDispatchers|BindEventtoEDTimeTick Event))

(fn FUnsubscribeTick
  (params (Event :type Delegate%20%28by%20ref%29))
  (EventDispatchers|UnbindEventfromEDTimeTick Event))

(fn FUnsubscribeAllTick
  (EventDispatchers|UnbindallEventsfromEDTimeTick))

(fn FIsDebug
  (return (Variables|Default|GetisDebug)))

(fn FInit
  (CallFunction|FDeleteOtherCameras))

(fn FDeleteOtherCameras
  (bind _outactors (Actor|GetAllActorsOfClass "/Script/Engine.CameraActor"))
  (for _array_element _outactors
    (if (not (Actor|ActorHasTag _array_element "GameplayCamera"))
      (Actor|DestroyActor _array_element))))

(fn FGetRoom
  (return (Variables|Default|GetRoom)))

(fn FSetRoom
  (params (Room :type BP%20Room%20Object%20Reference))
  (Variables|Default|SetRoom Room))

(fn FSetGameDifficult
  (params (GameDifficile :type E_GameDifficile%20Enum :default "NewEnumerator0"))
  (Variables|Default|SetGameDifficult GameDifficile))

(fn FGetGameDifficult
  (return (Variables|Default|GetGameDifficult)))

(fn FSetGameState
  (params (GameState :type E_GameState%20Enum :default "NewEnumerator0"))
  (Variables|Default|SetState GameState))

(fn FGetGameState
  (return (Variables|Default|GetState)))