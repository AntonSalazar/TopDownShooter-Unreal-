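; Player controller that relays movement and fire input to other objects through event dispatchers, with subscribe and unsubscribe wrapper functions.
; Move axes store and broadcast a combined input value, while the Fire axis broadcasts shoot whenever it is positive.
; Escape or Right Alt opens the HUD's gameplay menu unless the game state is the first enum value.
; EndPlay and Destroyed clear only the movement-input bindings, not the shoot bindings.
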(event EventEndPlay
  (params (EndPlayReason :type EEndPlayReason%20Enum :default "Destroyed"))
  (EDUpdateInputs|FUnsubscribeAllInputs))

(event EventDestroyed
  (EDUpdateInputs|FUnsubscribeAllInputs))

(event Input|AxisEvents|InputAxisMoveForward
  (params (AxisValue :type Float%20%28single-precision%29))
  (ED_UpdateInputs|FUpdateInputs (Math|Vector2D|MakeVector2D AxisValue (stale Input|AxisEvents|InputAxisMoveRight AxisValue))))

(event Input|AxisEvents|InputAxisMoveRight
  (params (AxisValue :type Float%20%28single-precision%29))
  (ED_UpdateInputs|FUpdateInputs (Math|Vector2D|MakeVector2D (stale Input|AxisEvents|InputAxisMoveForward AxisValue) AxisValue)))

(event Input|AxisEvents|InputAxisFire
  (params (AxisValue :type Float%20%28single-precision%29))
  (if (> AxisValue 0.0)
    (Default|CallEDShoot)))

(event Input|KeyboardEvents|Escape
  (params (Key :type Key%20Structure))
  (:Pressed
    (if (Utilities|Enum|NotEqual(Enum) (CallFunction|BPFLGetGameState) "NewEnumerator0")
      (Default|FShowGameplayMenu (CallFunction|BPFLGetHUD)))))

(event Input|KeyboardEvents|RightAlt
  (params (Key :type Key%20Structure))
  (:Pressed
    (if (Utilities|Enum|NotEqual(Enum) (CallFunction|BPFLGetGameState) "NewEnumerator0")
      (Default|FShowGameplayMenu (CallFunction|BPFLGetHUD)))))

(fn ConstructionScript)

(fn FUpdateInputs
  (params (Inputs :type Vector%202D%20Structure))
  (bind _output_get (Variables|Default|SetInputs Inputs))
  (Default|CallEDUpdateInputs _output_get))

(fn FSubscribeInputs
  (params (Event :type Delegate%20%28by%20ref%29))
  (EventDispatchers|BindEventtoEDUpdateInputs Event))

(fn FUnsubscribeInputs
  (params (Event :type Delegate%20%28by%20ref%29))
  (EventDispatchers|UnbindEventfromEDUpdateInputs Event))

(fn FUnsubscribeAllInputs
  (EventDispatchers|UnbindallEventsfromEDUpdateInputs))

(fn FSubscribeShoot
  (params (Event :type Delegate%20%28by%20ref%29))
  (EventDispatchers|BindEventtoEDShoot Event))

(fn FUnsubscribeShoot
  (params (Event :type Delegate%20%28by%20ref%29))
  (EventDispatchers|UnbindEventfromEDShoot Event))

(fn FUnsubscribeAllShoot
  (EventDispatchers|UnbindallEventsfromEDShoot))