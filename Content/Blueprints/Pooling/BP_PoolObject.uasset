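; Poolable actor for an object pool, which starts inactive on BeginPlay and is toggled by F_SetActive instead of being spawned or destroyed.
; F_SetActive sets visibility and ticking, then broadcasts ED_Active, whose own handler starts an optional LifeTime delay that deactivates the object.
; While active, Tick broadcasts ED_LifeCicle with the game state.
; Subscribe/unsubscribe wrappers expose both dispatchers, and EndPlay or Destroyed clears all bindings.
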(event Custom|ED_Active_Event
  (params (isActive :type Boolean))
  (if (and isActive (Variables|Default|GetUseLifeTime))
    (Utilities|MLifeCicle)))

(event EventBeginPlay
  (ED_Active|FSubscribeActive (delegate Custom|ED_Active_Event))
  (CallFunction|FSetActive false))

(event EventTick
  (params (DeltaSeconds :type Float%20%28single-precision%29))
  (Default|CallEDLifeCicle (CallFunction|BPFLGetGameState)))

(event EventEndPlay
  (params (EndPlayReason :type EEndPlayReason%20Enum :default "Destroyed"))
  (ED_Active|FUnsubscribeAllActive)
  (EDLifeCicle|FUnsubscribeAllLifeCicle))

(event EventDestroyed
  (ED_Active|FUnsubscribeAllActive)
  (EDLifeCicle|FUnsubscribeAllLifeCicle))

(fn ConstructionScript)

(fn FSubscribeActive
  (params (Event :type Delegate%20%28by%20ref%29))
  (EventDispatchers|BindEventtoEDActive Event))

(fn FUnsubscribeActive
  (params (Event :type Delegate%20%28by%20ref%29))
  (EventDispatchers|UnbindEventfromEDActive Event))

(fn FUnsubscribeAllActive
  (EventDispatchers|UnbindallEventsfromEDActive))

(fn FSubscribeLifeCicle
  (params (Event :type Delegate%20%28by%20ref%29))
  (EventDispatchers|BindEventtoEDLifeCicle Event))

(fn FUnsubscribeLifeCicle
  (params (Event :type Delegate%20%28by%20ref%29))
  (EventDispatchers|UnbindEventfromEDLifeCicle Event))

(fn FUnsubscribeAllLifeCicle
  (EventDispatchers|UnbindallEventsfromEDLifeCicle))

(fn FSetActive
  (params (isActive :type Boolean))
  (bind _output_get (Variables|Default|SetisActive isActive))
  (Rendering|SetActorHiddenInGame (Math|Boolean|NotEqual(Boolean) _output_get true))
  (Actor|Tick|SetActorTickEnabled _output_get)
  (Default|CallEDActive _output_get))