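; Object pool manager actor that prespawns configured BP_PoolObject actors on BeginPlay and hands them out for reuse.
; FSpawnPoolObject records each spawn in the nested category/object Pool array, renames it, and attaches it under a child actor named after its category.
; FGetPoolObject teleports and activates an inactive instance of the requested class, spawns another if none is found, and prints a debug warning for unregistered classes.
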(event EventBeginPlay
  (CallFunction|FPrespawn))

(fn ConstructionScript)

(fn FSpawnPoolObject
  (params (PoolObject :type BP%20Pool%20Object%20Class%20Reference) (CategoryIndex :type Integer) (ObjectIndex :type Integer) (Location :type Vector) (Rotation :type Rotator))
  (bind _childactors (Actor|GetAllChildActors false))
  (bind _pool (Variables|Default|GetPool))
  (bind _output (Utilities|Array|Get(acopy) _pool CategoryIndex))
  (bind (_name _objects) (Utilities|Struct|BreakSTR_PoolCategory _output))
  (bind _output_2 (Utilities|Array|Get(acopy) _objects ObjectIndex))
  (bind (_name_2 _object _count _onscene) (Utilities|Struct|BreakSTR_PoolSettings _output_2))
  (if (> (Utilities|Array|Length _childactors) CategoryIndex)
    (LocalVariables|SetCategory (Utilities|Array|Get(acopy) _childactors CategoryIndex))
    (else
      (bind _returnvalue (AddComponent|AddChildActorComponent true))
      (bind _output_get (LocalVariables|SetCategory (Variables|/Script/Engine.ChildActorComponent|GetChildActor _returnvalue)))))
  (bind _returnvalue_2 (Game|SpawnActorfromClass PoolObject (Math|Transform|MakeTransform Location Rotation) "AlwaysSpawn" 0 0))
  (LocalVariables|SetCategory (Class|FLHelper|RenameObject _name _output_get))
  (bind _asbp_pool_object (Utilities|Casting|CastToBP_PoolObject (Class|FLHelper|RenameObject (Utilities|String|Append _name_2 "_" (Utilities|String|ToString(Integer) (Utilities|Array|Length _onscene))) _returnvalue_2)))
  (Utilities|Array|Add _onscene _asbp_pool_object)
  (Utilities|Array|SetArrayElem _objects ObjectIndex (Utilities|Struct|MakeSTR_PoolSettings _name_2 _object _count _onscene) true)
  (Transformation|AttachActorToActor _returnvalue_2 (LocalVariables|GetCategory) "None" "KeepRelative" "KeepRelative" "KeepRelative" true)
  (Utilities|Array|SetArrayElem (Variables|Default|GetPool) CategoryIndex (Utilities|Struct|MakeSTR_PoolCategory _name _objects) true)
  (return _returnvalue_2))

(fn FGetPoolObject
  (params (PoolObject :type BP%20Pool%20Object%20Class%20Reference) (Location :type Vector) (Rotation :type Rotator))
  (bind (_array_element _array_index) (Utilities|Array|ForEachLoopwithBreak (Variables|Default|GetPool) :!label _label)
    (:LoopBody
      (bind (_array_element_2 _array_index_2) (Utilities|Array|ForEachLoopwithBreak (.Objects (Utilities|Struct|BreakSTR_PoolCategory _array_element)) :!label _label_2)
        (:LoopBody
          (if (== (.Object (Utilities|Struct|BreakSTR_PoolSettings _array_element_2)) PoolObject)
            (LocalVariables|SetFindedIndexCategory _array_index)
            (LocalVariables|SetFindedIndexObject _array_index_2)
            (bind _array_element_3 (Utilities|Array|ForEachLoopwithBreak (.OnScene (Utilities|Struct|BreakSTR_PoolSettings _array_element_2)) :!label _label_3)
              (:LoopBody
                (if (not (Variables|/Game/Blueprints/Pooling/BP_PoolObject.BP_PoolObject_C|GetisActive _array_element_3))
                  (LocalVariables|SetisFinded true)
                  (goto _label_3 Break)))
              (:Completed
                (goto _label_2 Break)))))
        (:Completed
          (if (LocalVariables|GetisFinded)
            (goto _label Break)))))
    (:Completed
      (if (LocalVariables|GetisFinded)
        (Transformation|SetActorLocationAndRotation _array_element_3 Location Rotation false true)
        (Default|FSetActive _array_element_3 true)
        (return _array_element_3)
        (elif (and (!= (LocalVariables|GetFindedIndexCategory) -1) (!= (LocalVariables|GetFindedIndexObject) -1))
          (bind _return (CallFunction|FSpawnPoolObject PoolObject (LocalVariables|GetFindedIndexCategory) (LocalVariables|GetFindedIndexObject) Location Rotation))
          (Default|FSetActive _return true)
          (return _return)
          (elif (CallFunction|BPFLIsDebug)
            (Development|PrintText (Utilities|Text|FormatText "Element {element} NOT FOUNDED!" (Utilities|Text|ToText(String) (Utilities|GetClassDisplayName PoolObject))) true true "(R=1.000000,G=0.000000,B=0.000000,A=1.000000)" 5.0)))))))

(fn FPrespawn
  (for (_array_element _array_index) (Variables|Default|GetPool)
    (for (_array_element_2 _array_index_2) (.Objects (Utilities|Struct|BreakSTR_PoolCategory _array_element))
      (for _index (range 0 (- (.Count (Utilities|Struct|BreakSTR_PoolSettings _array_element_2)) 1))
        (CallFunction|FSpawnPoolObject (.Object (Utilities|Struct|BreakSTR_PoolSettings _array_element_2)) _array_index _array_index_2 "0, 0, 0" "0, 0, 0")))))