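; Base character for both the player and AI enemies, switched by IsPlayer, with difficulty-based speed and fire rate.
; Player movement and shooting come from controller dispatchers, while AI runs on the GameMode tick, using sphere-trace avoidance, chasing, and shooting on clear line of sight.
; Shots draw pooled projectiles behind a fire-rate delay.
; It registers with the room, and death triggers camera shake, team-colored explosion and a replacement spawn request.
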(event Custom|ED_Inputs
  (params (Inputs :type Vector%202D%20Structure))
  (if (Utilities|Enum|Equal(Enum) (CallFunction|BPFLGetGameState) "NewEnumerator2")
    (Settings|FMovement (Math|Vector|MakeVector (.x Inputs) (.y Inputs) 0.0))))

(event Custom|ED_Tick
  (params (GameState :type E_GameState%20Enum :default "NewEnumerator0"))
  (if (Utilities|Enum|Equal(Enum) GameState "NewEnumerator2")
    (if (not (Variables|Settings|GetisPlayer))
      (Utilities|MAICollision)
      (if (not (Variables|Settings|GetColliside))
        (Utilities|MAILogic)))
    (elif (Utilities|Enum|Equal(Enum) GameState "NewEnumerator0")
      (Actor|DestroyActor))))

(event Custom|ED_Shoot
  (if (Utilities|Enum|Equal(Enum) (CallFunction|BPFLGetGameState) "NewEnumerator2")
    (Utilities|MShoot)))

(event Custom|Event_Die
  (bind _returnvalue (Transformation|GetActorLocation))
  (bind _returnvalue_2 (Transformation|GetActorRotation))
  (bind _isplayer (Variables|Settings|GetisPlayer))
  (Camera|PlayWorldCameraShake "/Game/Blueprints/Main/BP_CameraShake.BP_CameraShake_C" (Transformation|GetActorLocation) 0.0 5e+03)
  (Default|FSpawnCharacter (CallFunction|BPFLGetRoom) _isplayer)
  (if _isplayer
    (Effects|SpawnEmitteratLocation "/Game/GameResources/Particles/PS_ExplosionBlue.PS_ExplosionBlue" _returnvalue _returnvalue_2)
    (else
      (Effects|SpawnEmitteratLocation "/Game/GameResources/Particles/PS_ExplosionRed.PS_ExplosionRed" _returnvalue _returnvalue_2)))
  (Actor|DestroyActor))

(event EventBeginPlay
  (Settings|FInit (delegate Custom|ED_Inputs) (delegate Custom|ED_Shoot) (delegate Custom|ED_Tick)))

(event EventEndPlay
  (params (EndPlayReason :type EEndPlayReason%20Enum :default "Destroyed"))
  (Settings|FDeinit (delegate Custom|ED_Inputs) (delegate Custom|ED_Shoot) (delegate Custom|ED_Tick)))

(fn ConstructionScript)

(fn FInit
  (params (ED_Inputs :type Delegate%20%28by%20ref%29) (ED_Shoot :type Delegate%20%28by%20ref%29) (ED_Tick :type Delegate%20%28by%20ref%29))
  (ED_Inputs|FSubscribeInputs ED_Inputs)
  (ED_Shoot|FSubscribeShoot ED_Shoot)
  (Default|FSubscribeTick (CallFunction|BPFLGetGameMode) ED_Tick)
  (Rendering|Material|SetMaterial (Variables|Default|GetMesh) 0 (Variables|Settings|GetMaterial))
  (Default|FAddCharacter (CallFunction|BPFLGetRoom) self)
  (CallFunction|FSetSettings))

(fn FDeinit
  (params (ED_Inputs :type Delegate%20%28by%20ref%29) (ED_Shoot :type Delegate%20%28by%20ref%29) (ED_Tick :type Delegate%20%28by%20ref%29))
  (EDInputs|FUnsubscribeInputs ED_Inputs)
  (ED_Shoot|FUnsubscribeShoot ED_Shoot)
  (Default|FUnsubscribeTick (CallFunction|BPFLGetGameMode) ED_Tick)
  (Default|FRemoveCharacter (CallFunction|BPFLGetRoom) self))

(fn FSubscribeInputs
  (params (ED_Inputs :type Delegate%20%28by%20ref%29))
  (if (Variables|Settings|GetisPlayer)
    (bind _asbp_player_controller (Utilities|Casting|CastToBP_PlayerController (Game|GetPlayerController 0)))
    (Default|FSubscribeInputs _asbp_player_controller ED_Inputs)))

(fn FUnsubscribeInputs
  (params (ED_Inputs :type Delegate%20%28by%20ref%29))
  (if (Variables|Settings|GetisPlayer)
    (bind _asbp_player_controller (Utilities|Casting|CastToBP_PlayerController (Game|GetPlayerController 0)))
    (Default|FUnsubscribeInputs _asbp_player_controller ED_Inputs)))

(fn FMovement
  (params (Direction :type Vector))
  (bind _returnvalue (Utilities|Time|GetWorldDeltaSeconds))
  (if (> (Math|Vector|VectorLength Direction) 0.0)
    (Transformation|SetWorldRotation (Variables|Default|GetMesh) (Math|Interpolation|RInterpTo (Transformation|GetWorldRotation (Variables|Default|GetMesh)) (Math|Conversions|RotationFromXVector Direction) _returnvalue 5.0) false false)
    (bind _sweephitresult (Transformation|AddActorWorldOffset (* (Transformation|GetActorForwardVector) (* (Variables|Settings|GetMoveSpeed) _returnvalue)) (Math|Boolean|NotEqual(Boolean) (Variables|Settings|GetisPlayer) false)))
    (if (.bBlockingHit (Collision|BreakHitResult _sweephitresult))
      (Transformation|AddActorWorldOffset (* (Math|Vector|Normalize (Math|Vector|MakeVector (.X (Math|Vector|BreakVector (.Normal (Collision|BreakHitResult _sweephitresult)))) (.Y (Math|Vector|BreakVector (.Normal (Collision|BreakHitResult _sweephitresult)))) 0.0)) (- 1.0 (.Time (Collision|BreakHitResult _sweephitresult)))) true))))

(fn FSubscribeShoot
  (params (ED_Shoot :type Delegate%20%28by%20ref%29))
  (if (Variables|Settings|GetisPlayer)
    (bind _asbp_player_controller (Utilities|Casting|CastToBP_PlayerController (Game|GetPlayerController 0)))
    (Default|FSubscribeShoot _asbp_player_controller ED_Shoot)))

(fn FUnsubscribeShoot
  (params (ED_Shoot :type Delegate%20%28by%20ref%29))
  (if (Variables|Settings|GetisPlayer)
    (bind _asbp_player_controller (Utilities|Casting|CastToBP_PlayerController (Game|GetPlayerController 0)))
    (Default|FUnsubscribeShoot _asbp_player_controller ED_Shoot)))

(fn FAIVectors
  (Variables|Settings|SetVector (+ (Transformation|GetActorLocation) (* (Transformation|GetActorForwardVector) 5e+01))))

(fn FIsPlayer
  (return (Variables|Settings|GetisPlayer)))

(fn FSetSettings
  (bind _isplayer (Variables|Settings|GetisPlayer))
  (switch Utilities|FlowControl|Switch|SwitchonE_GameDifficile (CallFunction|BPFLGetGameDifficult)
    (:NewEnumerator0
      (if _isplayer
        (Variables|Settings|SetMoveSpeed 3e+02)
        (Variables|Shoot|SetFireRate 0.15)
        (else
          (Variables|Settings|SetMoveSpeed 2e+02)
          (Variables|Shoot|SetFireRate 1.75))))
    (:NewEnumerator1
      (if _isplayer
        (Variables|Settings|SetMoveSpeed 2.5e+02)
        (Variables|Shoot|SetFireRate 0.35)
        (else
          (Variables|Settings|SetMoveSpeed 3.5e+02)
          (Variables|Shoot|SetFireRate 0.95))))
    (:NewEnumerator2
      (if _isplayer
        (Variables|Settings|SetMoveSpeed 2e+02)
        (Variables|Shoot|SetFireRate 0.45)
        (else
          (Variables|Settings|SetMoveSpeed 4.5e+02)
          (Variables|Shoot|SetFireRate 0.5))))))